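; BP_HumanoidEnemy is a humanoid enemy Blueprint that shows a boss-style health display while it is targeted.
; When targeted, it creates a WB_BossInfo widget, adds it to the viewport and initializes its health bar with the enemy's StatsComponent.
; When untargeted, it removes that widget through the GameViewportSubsystem.
; BeginPlay and the construction script only call the parent, and OnTargeted extends the parent's handling.
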(event `self.ReceiveBeginPlay`
  (`parent.ReceiveBeginPlay`))

(event `/Game/CombatSystem/Blueprints/Interfaces/Targeting_BPI.OnTargeted`
  (params (`bIsTargeted?` :type Boolean))
  (`parent.OnTargeted` `bIsTargeted?`)
  (if `bIsTargeted?`
    (bind _returnvalue (`|CreateWidget` "/Game/CombatSystem/UI/WB_BossInfo.WB_BossInfo_C"))
    (bind _output_get (set `self.BossInfoWidget` _returnvalue))
    (`UserWidget.AddToViewport` _output_get 0)
    (`/Game/CombatSystem/UI/WB_HealthBar.Initialize` (`/Game/CombatSystem/UI/WB_BossInfo.WB_BossHealthBar` (`self.BossInfoWidget`)) (`self.StatsComponent`))
    (else
      (`GameViewportSubsystem.RemoveWidget` (subsystem `GameViewportSubsystem`) (`self.BossInfoWidget`)))))

(fn `UserConstructionScript`
  (`parent.UserConstructionScript`))